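; BP_X02 is an actor that drives level interaction through mouse hover and a key press, showing the cursor on BeginPlay.
; Each tick it traces under the cursor and sends HoverMessage to hit actors implementing InteractableInterface.
; Pressing F runs a small sphere overlap at its own location and calls InteractMessage on the first InteractableBase found.
; Hover is interface-based, while interaction relies on a cast to the base class.
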(event `self.ReceiveBeginPlay`
  (set `PlayerController.bShowMouseCursor` true (`GameplayStatics.GetPlayerController` 0)))

(event `self.ReceiveTick`
  (params (DeltaSeconds :type "Float (single-precision)"))
  (`self.Hover_Player`))

(event `Key|F`
  (params (Key :type "Key Structure"))
  (:`Pressed`
    (bind _outactors (`KismetSystemLibrary.SphereOverlapActors` (`self.K2_GetActorLocation`) 42.0 (`self.Object Types`)))
    (for _array_element _outactors
      (bind _asinteractable_base (cast `InteractableBase` _array_element))
      (message `InteractableInterface.Interact` _asinteractable_base)
      (break))))

(event `Hover_Player`
  (bind (_hitresult _returnvalue) (`PlayerController.GetHitResultUnderCursorForObjects` (`GameplayStatics.GetPlayerController` 0) (`self.Object Types`) true))
  (if _returnvalue
    (if (`KismetSystemLibrary.DoesImplementInterface` (`.HitActor` (`GameplayStatics.BreakHitResult` _hitresult)) "/Script/ReTri.InteractableInterface")
      (message `InteractableInterface.Hover` (`.HitActor` (`GameplayStatics.BreakHitResult` _hitresult))))))

(fn `UserConstructionScript`)