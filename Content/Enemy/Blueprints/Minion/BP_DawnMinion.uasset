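; BP_DawnMinion is an enemy minion Blueprint that tracks its health and shows it on a health bar widget.
; On AnyDamage it subtracts the damage from CurrentHP, clamped between zero and MaxHP.
; It then casts its Widget component's user widget to WBP_MinionHP and sets the HPbar percent to the health ratio.
; It contains no death handling, and BeginPlay and the construction script are empty.
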(event `self.ReceiveBeginPlay`)

(event `self.ReceiveAnyDamage`
  (params (Damage :type "Float (single-precision)") (DamageType :type "DamageType Object Reference") (InstigatedBy :type "Controller Object Reference") (DamageCauser :type "Actor Object Reference"))
  (set `self.CurrentHP` (`KismetMathLibrary.FClamp` (- (`self.CurrentHP`) Damage) 0.0 (`self.MaxHP`)))
  (bind _aswbp_minion_hp (cast `/Game/Enemy/UI/WBP_MinionHP` (`WidgetComponent.GetUserWidgetObject` (`self.Widget`))))
  (`ProgressBar.SetPercent` (`/Game/Enemy/UI/WBP_MinionHP.HPbar` _aswbp_minion_hp) (/ (`self.CurrentHP`) (`self.MaxHP`))))

(fn `UserConstructionScript`)